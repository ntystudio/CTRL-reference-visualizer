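; BP_CRV_TestActor is a sample-map test actor for working with references to AC_CRV_TestComponent.
; Its construction script labels the actor by writing its display name to a TextRender.
; SetComponentFromActor stores the AC_CRV_TestComponent found on ActorRef in ComponentRef, then clears ActorRef, turning an actor reference into a component reference.
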(event Custom|SetComponentFromActor
  (Variables|Default|SetComponentRef (Actor|GetComponentbyClass (Variables|Default|GetActorRef) "/CtrlReferenceVisualizer/Sample_Maps/SampleAssets/AC_CRV_TestComponent.AC_CRV_TestComponent_C"))
  (Variables|Default|SetActorRef 0))

(fn ConstructionScript
  (|CallParentFunction)
  (Rendering|Components|TextRender|SetText (Variables|Default|GetTextRender) (Utilities|Text|ToText(String) (Utilities|GetDisplayName self))))